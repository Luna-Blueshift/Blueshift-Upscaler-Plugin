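; Game setting Blueprint for toggling upscaler frame generation.
; It reads and writes the desired frame generation value through the Blueshift upscaler subsystem.
; Its visibility is Enabled only when the subsystem reports frame generation support for the currently desired upscaler, otherwise Disabled.
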(event EventSetValue
  (params (Value :type Boolean))
  (Class|BlueshiftUpscalerSubsystem|SetDesiredFrameGen (|BlueshiftUpscalerSubsystem) Value))

(fn GetVisibility
  (bind _returnvalue (|BlueshiftUpscalerSubsystem))
  (return (select (Class|BlueshiftUpscalerSubsystem|IsFrameGenSupported _returnvalue (Class|BlueshiftUpscalerSubsystem|GetDesiredUpscaler _returnvalue)) "Enabled" "Disabled")))

(fn GetValue
  (return (Class|BlueshiftUpscalerSubsystem|GetDesiredFrameGen (|BlueshiftUpscalerSubsystem))))