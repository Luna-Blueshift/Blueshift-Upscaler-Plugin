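; Game setting Blueprint for the DLSS RR toggle, backed by the Blueshift IQ manager.
; SetValue passes the chosen value to the manager's SetDLSSRREnabled.
; GetVisibility hides the setting unless DLSS is the desired upscaler, and disables it when DLSS RR is unsupported.
; GetValue returns whether DLSS RR is supported, rather than reading back an enabled state.
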(event EventSetValue
  (params (Value :type Boolean))
  (Class|BlueshiftIQManager|SetDLSSRREnabled (|BlueshiftIQManager) Value))

(fn GetVisibility
  (bind _returnvalue (|BlueshiftIQManager))
  (if (Utilities|Enum|Equal(Enum) (Class|BlueshiftIQManager|GetDesiredUpscaler _returnvalue) "DLSS")
    (return (select (Class|BlueshiftIQManager|IsDLSSRRSupported _returnvalue) "Enabled" "Disabled"))
    (else
      (return "Hidden"))))

(fn GetValue
  (return (Class|BlueshiftIQManager|IsDLSSRRSupported (|BlueshiftIQManager))))