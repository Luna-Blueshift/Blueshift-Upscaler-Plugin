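; Game setting Blueprint that exposes FSR sharpness as a ranged numeric option.
; It reads and writes the value through the Blueshift upscaler subsystem, within a fixed range.
; The setting is shown only when FSR is the desired upscaler and is hidden otherwise.
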(event EventSetValue
  (params (Value :type Float%20%28single-precision%29))
  (Class|BlueshiftUpscalerSubsystem|SetFSRSharpness (|BlueshiftUpscalerSubsystem) Value))

(fn GetValueRange
  (return 0.0 2e+01))

(fn GetValue
  (return (Class|BlueshiftUpscalerSubsystem|GetFSRSharpness (|BlueshiftUpscalerSubsystem))))

(fn GetVisibility
  (return (select (Utilities|Enum|Equal(Enum) (Class|BlueshiftUpscalerSubsystem|GetDesiredUpscaler (|BlueshiftUpscalerSubsystem)) "FSR") "Enabled" "Hidden")))