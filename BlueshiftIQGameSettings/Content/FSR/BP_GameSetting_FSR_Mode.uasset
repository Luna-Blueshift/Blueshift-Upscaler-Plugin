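; Game setting Blueprint for choosing the FSR mode, from Native AA through Ultra Performance.
; It reads and writes the mode through the BlueshiftIQManager and supplies the options as a map of values to labels.
; The setting is enabled only when the manager's desired upscaler is FSR, and is hidden otherwise.
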(event EventSetValue
  (params (Value :type Integer))
  (Class|BlueshiftIQManager|SetFSRMode (|BlueshiftIQManager) Value))

(fn GetValue
  (return (Class|BlueshiftIQManager|GetFSRMode (|BlueshiftIQManager))))

(fn GetVisibility
  (return (select (Utilities|Enum|Equal(Enum) (Class|BlueshiftIQManager|GetDesiredUpscaler (|BlueshiftIQManager)) "FSR") "Enabled" "Hidden")))

(fn GetOptions
  (return (Utilities|Map|MakeMap 0 "Native AA" 1 "Quality" 2 "Balanced" 3 "Performance" 4 "Ultra Performance")))