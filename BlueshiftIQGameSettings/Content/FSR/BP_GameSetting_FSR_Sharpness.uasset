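; A game setting Blueprint that exposes AMD FSR sharpness as an adjustable numeric value with a fixed range.
; It reads and writes the value directly through the Blueshift IQ Manager.
; The setting is enabled only when the manager's desired upscaler is FSR, and is hidden otherwise.
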(event EventSetValue
  (params (Value :type Float%20%28single-precision%29))
  (Class|BlueshiftIQManager|SetFSRSharpness (|BlueshiftIQManager) Value))

(fn GetValueRange
  (return 0.0 2e+01))

(fn GetValue
  (return (Class|BlueshiftIQManager|GetFSRSharpness (|BlueshiftIQManager))))

(fn GetVisibility
  (return (select (Utilities|Enum|Equal(Enum) (Class|BlueshiftIQManager|GetDesiredUpscaler (|BlueshiftIQManager)) "FSR") "Enabled" "Hidden")))