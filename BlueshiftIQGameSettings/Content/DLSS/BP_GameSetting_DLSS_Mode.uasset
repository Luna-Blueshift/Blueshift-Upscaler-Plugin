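; Game setting Blueprint for choosing the DLSS mode.
; It reads and writes the mode through the BlueshiftIQManager and offers a fixed map of labeled options from Auto and DLAA through Ultra Performance.
; The setting is visible and enabled only when the manager's desired upscaler is DLSS, and is hidden otherwise.
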(event EventSetValue
  (params (Value :type Integer))
  (Class|BlueshiftIQManager|SetDLSSMode (|BlueshiftIQManager) Value))

(fn GetValue
  (return (Class|BlueshiftIQManager|GetDLSSMode (|BlueshiftIQManager))))

(fn GetVisibility
  (return (select (Utilities|Enum|Equal(Enum) (Class|BlueshiftIQManager|GetDesiredUpscaler (|BlueshiftIQManager)) "DLSS") "Enabled" "Hidden")))

(fn GetOptions
  (return (Utilities|Map|MakeMap 1 "Auto" 2 "DLAA" 3 "Ultra Quality" 4 "Quality" 5 "Balanced" 6 "Performance" 7 "Ultra Performance")))