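; Game setting Blueprint that toggles frame generation through the Blueshift IQ manager.
; SetValue and GetValue write and read the manager's desired frame generation state.
; GetVisibility disables the setting when the currently desired upscaler does not support frame generation.
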(event EventSetValue
  (params (Value :type Boolean))
  (Class|BlueshiftIQManager|SetDesiredFrameGen (|BlueshiftIQManager) Value))

(fn GetVisibility
  (bind _returnvalue (|BlueshiftIQManager))
  (return (select (Class|BlueshiftIQManager|IsFrameGenSupported _returnvalue (Class|BlueshiftIQManager|GetDesiredUpscaler _returnvalue)) "Enabled" "Disabled")))

(fn GetValue
  (return (Class|BlueshiftIQManager|GetDesiredFrameGen (|BlueshiftIQManager))))