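; Game setting Blueprint that exposes the XeSS upscaler quality mode as a selectable option.
; It reads and writes the value through the Blueshift upscaler subsystem and maps mode indices to display names from Ultra Performance to AA.
; The setting is shown only while XeSS is the desired upscaler and is hidden otherwise.
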(event EventSetValue
  (params (Value :type Integer))
  (Class|BlueshiftUpscalerSubsystem|SetXeSSQualityMode (|BlueshiftUpscalerSubsystem) Value))

(fn GetValue
  (return (Class|BlueshiftUpscalerSubsystem|GetXeSSQualityMode (|BlueshiftUpscalerSubsystem))))

(fn GetVisibility
  (return (select (Utilities|Enum|Equal(Enum) (Class|BlueshiftUpscalerSubsystem|GetDesiredUpscaler (|BlueshiftUpscalerSubsystem)) "XeSS") "Enabled" "Hidden")))

(fn GetOptions
  (return (Utilities|Map|MakeMap 1 "Ultra Performance" 2 "Performance" 3 "Balanced" 4 "Quality" 5 "Ultra Quality" 6 "Ultra Quality+" 7 "AA")))