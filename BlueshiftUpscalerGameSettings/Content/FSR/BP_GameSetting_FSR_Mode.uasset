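; Game setting Blueprint for choosing the FSR upscaling quality mode, from Native AA through Ultra Performance.
; It reads and writes the mode through BlueshiftUpscalerSubsystem and supplies the integer-keyed option labels.
; The setting is visible only while FSR is the desired upscaler, and hidden otherwise.
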(event EventSetValue
  (params (Value :type Integer))
  (Class|BlueshiftUpscalerSubsystem|SetFSRMode (|BlueshiftUpscalerSubsystem) Value))

(fn GetValue
  (return (Class|BlueshiftUpscalerSubsystem|GetFSRMode (|BlueshiftUpscalerSubsystem))))

(fn GetVisibility
  (return (select (Utilities|Enum|Equal(Enum) (Class|BlueshiftUpscalerSubsystem|GetDesiredUpscaler (|BlueshiftUpscalerSubsystem)) "FSR") "Enabled" "Hidden")))

(fn GetOptions
  (return (Utilities|Map|MakeMap 0 "Native AA" 1 "Quality" 2 "Balanced" 3 "Performance" 4 "Ultra Performance")))