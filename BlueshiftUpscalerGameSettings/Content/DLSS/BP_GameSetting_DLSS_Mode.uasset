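; Game setting Blueprint that exposes the DLSS quality mode as a selectable option.
; It reads and writes the mode through the Blueshift Upscaler Subsystem and offers a fixed map of choices from Auto and DLAA to Ultra Performance.
; The setting is enabled only while DLSS is the desired upscaler and is hidden otherwise.
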(event EventSetValue
  (params (Value :type Integer))
  (Class|BlueshiftUpscalerSubsystem|SetDLSSMode (|BlueshiftUpscalerSubsystem) Value))

(fn GetValue
  (return (Class|BlueshiftUpscalerSubsystem|GetDLSSMode (|BlueshiftUpscalerSubsystem))))

(fn GetVisibility
  (return (select (Utilities|Enum|Equal(Enum) (Class|BlueshiftUpscalerSubsystem|GetDesiredUpscaler (|BlueshiftUpscalerSubsystem)) "DLSS") "Enabled" "Hidden")))

(fn GetOptions
  (return (Utilities|Map|MakeMap 1 "Auto" 2 "DLAA" 3 "Ultra Quality" 4 "Quality" 5 "Balanced" 6 "Performance" 7 "Ultra Performance")))