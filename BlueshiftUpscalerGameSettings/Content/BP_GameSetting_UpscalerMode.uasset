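; A game setting Blueprint that lets the player choose the upscaler mode (DLSS, FSR, XeSS or None).
; It reads and writes the desired upscaler through the BlueshiftUpscalerSubsystem, converting between integer option values and the upscaler enum.
; The option list is built at runtime from the subsystem's supported upscalers mapped to display names, with None always added.
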(event EventSetValue
  (params (Value :type Integer))
  (Class|BlueshiftUpscalerSubsystem|SetDesiredUpscaler (|BlueshiftUpscalerSubsystem) (Utilities|Enum|ByteToEnumEBlueshiftUpscalerMode (Math|Conversions|ToByte(Integer) Value))))

(fn GetValue
  (return (Math|Conversions|ToInteger(Byte) (Class|BlueshiftUpscalerSubsystem|GetDesiredUpscaler (|BlueshiftUpscalerSubsystem)))))

(fn GetOptions
  (bind _result (LocalVariables|GetResult))
  (LocalVariables|SetOptions (Utilities|Map|MakeMap 1 "DLSS" 2 "FSR" 3 "XeSS"))
  (bind _returnvalue (Class|BlueshiftUpscalerSubsystem|GetSupportedUpscalers (|BlueshiftUpscalerSubsystem)))
  (for _array_element _returnvalue
    (bind (_value _returnvalue_2) (Utilities|Map|Find (LocalVariables|GetOptions) (Math|Conversions|ToInteger(Byte) _array_element)))
    (if _returnvalue_2
      (Utilities|Map|Add (LocalVariables|GetResult) (Math|Conversions|ToInteger(Byte) _array_element) _value)))
  (Utilities|Map|Add _result 0 "None")
  (return _result))