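; Game setting Blueprint that exposes the anti-aliasing method as a selectable option.
; SetValue and GetValue convert between the option's integer and the Blueshift AA method enum, writing and reading it through the BlueshiftIQManager.
; GetOptions filters a fixed table of method labels down to the manager's supported AA methods, so only those are offered.
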(event EventSetValue
  (params (Value :type Integer))
  (Class|BlueshiftIQManager|SetAAMethod (|BlueshiftIQManager) (Utilities|Enum|ByteToEnumEBlueshiftAAMethod (Math|Conversions|ToByte(Integer) Value))))

(fn GetValue
  (return (Math|Conversions|ToInteger(Byte) (Class|BlueshiftIQManager|GetAAMethod (|BlueshiftIQManager)))))

(fn GetOptions
  (LocalVariables|SetOptions (Utilities|Map|MakeMap 0 "None" 1 "FXAA" 2 "TAA" 3 "MSAA" 4 "TSR" 5 "SMAA"))
  (bind _returnvalue (Class|BlueshiftIQManager|GetSupportedAAMethods (|BlueshiftIQManager)))
  (for _array_element _returnvalue
    (bind (_value _returnvalue_2) (Utilities|Map|Find (LocalVariables|GetOptions) (Math|Conversions|ToInteger(Byte) _array_element)))
    (if _returnvalue_2
      (Utilities|Map|Add (LocalVariables|GetResult) (Math|Conversions|ToInteger(Byte) _array_element) _value)))
  (return (LocalVariables|GetResult)))