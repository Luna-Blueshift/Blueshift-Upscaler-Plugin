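; Game setting Blueprint for toggling DLSS Ray Reconstruction (RR) through the Blueshift upscaler subsystem.
; Its getter and setter read and write the subsystem's RR enabled state directly.
; Visibility hides the setting unless DLSS is the desired upscaler, then enables or disables it based on whether RR is supported.
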(event EventSetValue
  (params (Value :type Boolean))
  (Class|BlueshiftUpscalerSubsystem|SetDLSSRREnabled (|BlueshiftUpscalerSubsystem) Value))

(fn GetVisibility
  (bind _returnvalue (|BlueshiftUpscalerSubsystem))
  (if (Utilities|Enum|Equal(Enum) (Class|BlueshiftUpscalerSubsystem|GetDesiredUpscaler _returnvalue) "DLSS")
    (return (select (Class|BlueshiftUpscalerSubsystem|IsDLSSRRSupported _returnvalue) "Enabled" "Disabled"))
    (else
      (return "Hidden"))))

(fn GetValue
  (return (Class|BlueshiftUpscalerSubsystem|GetDLSSRREnabled (|BlueshiftUpscalerSubsystem))))